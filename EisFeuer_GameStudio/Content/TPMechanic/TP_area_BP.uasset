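; Teleport area that reveals a portal and sends the game to another level once all collectables are gathered.
; Any overlap with its Box checks that the game mode's CollectablesLeft is zero, then shows the Portal.
; After a short delay it stores its PortalID in the game instance and opens the level named by its Destination enum.
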(event `self.Box.OnComponentBeginOverlap`
  (params (OverlappedComponent :type "PrimitiveComponent Object Reference") (OtherActor :type "Actor Object Reference") (OtherComp :type "PrimitiveComponent Object Reference") (OtherBodyIndex :type Integer) (bFromSweep :type Boolean) (SweepResult :type "HitResult Structure (by ref)"))
  (bind _asthird_person_game_mode (cast `/Game/ThirdPersonBP/Blueprints/ThirdPersonGameMode` (`GameplayStatics.GetGameMode`)))
  (if (== (`/Game/ThirdPersonBP/Blueprints/ThirdPersonGameMode.Collectables_Left` _asthird_person_game_mode) 0)
    (`SceneComponent.SetVisibility` (`self.Portal`) true false)
    (`KismetSystemLibrary.Delay` 5.0)
    (bind _asmy_game_instance (cast `/Game/TPMechanic/MyGameInstance` (`GameplayStatics.GetGameInstance`)))
    (set `/Game/TPMechanic/MyGameInstance.PortalID` (`self.PortalID`) _asmy_game_instance)
    (`GameplayStatics.OpenLevel` (`KismetStringLibrary.Conv_StringToName` (`|GetEnumeratorNameAsString` (`self.Destination`))))))

(fn `UserConstructionScript`)